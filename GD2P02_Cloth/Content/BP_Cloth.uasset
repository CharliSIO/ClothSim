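; BP_Cloth is a cloth actor with keyboard-driven wind controls and a HUD widget that receives a reference to it.
; Left/Right set a yaw rotation rate and Up/Down set a wind strength acceleration, each zeroed on release.
; Tick integrates both rates into WindAngle and WindStrength, then rotates and scales an arrow to visualize the wind.
; K calls DropCloth, whose logic is defined outside these graphs.
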(event `self.ReceiveBeginPlay`
  (bind _returnvalue (`|CreateWidget` "/Game/WBP_HUDWidget.WBP_HUDWidget_C" null self))
  (bind _output_get (set `self.HUDWidget` _returnvalue))
  (`UserWidget.AddToViewport` _output_get 0))

(event `Key|K`
  (params (Key :type "Key Structure"))
  (:`Pressed`
    (`self.DropCloth`)))

(event `Key|Right`
  (params (Key :type "Key Structure"))
  (:`Pressed`
    (`KismetSystemLibrary.PrintString` "Pressed Right")
    (set `self.RotationRate` 90.0))
  (:`Released`
    (set `self.RotationRate` 0.0 :!label _label)))

(event `Key|Up`
  (params (Key :type "Key Structure"))
  (:`Pressed`
    (set `self.WindAcceleration` 30.0))
  (:`Released`
    (set `self.WindAcceleration` 0.0 :!label _label_2)))

(event `Key|Down`
  (params (Key :type "Key Structure"))
  (:`Pressed`
    (set `self.WindAcceleration` -30.0))
  (:`Released`
    (goto _label_2)))

(event `Key|Left`
  (params (Key :type "Key Structure"))
  (:`Pressed`
    (`KismetSystemLibrary.PrintString` "Pressed Left")
    (set `self.RotationRate` -90.0))
  (:`Released`
    (goto _label)))

(event `self.ReceiveTick`
  (params (DeltaSeconds :type "Float (single-precision)"))
  (bind (_windangle_roll _windangle_pitch _windangle_yaw) (`KismetMathLibrary.BreakRotator` (`self.WindAngle`)))
  (bind _output_get (set `self.WindAngle` (`KismetMathLibrary.MakeRotator` _windangle_roll _windangle_pitch (+ _windangle_yaw (* DeltaSeconds (`self.RotationRate`))))))
  (`SceneComponent.K2_SetWorldRotation` (`self.ArrowOrigin`) _output_get false false)
  (bind _output_get_2 (set `self.WindStrength` (+ (`self.WindStrength`) (* DeltaSeconds (`self.WindAcceleration`)))))
  (set `ArrowComponent.ArrowLength` (* _output_get_2 3.0) (`self.Arrow`)))

(fn `UserConstructionScript`)